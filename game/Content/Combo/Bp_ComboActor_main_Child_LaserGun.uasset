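; Laser gun combo actor, a child variant of the main combo actor, that plays a one-shot animation and then destroys itself.
; PlayAnim plays a 2D laser sound and starts a timeline whose track slides the static mesh along X within a clamped range while pitching it.
; Once the track passes a threshold it activates the Niagara effect, and the actor is destroyed when the timeline finishes.
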(event `self.PlayAnim`
  (`GameplayStatics.PlaySound2D` "/Game/music/Sound/laser.laser" 1.0 1.0 0.0 null null)
  (bind (_direction _newtrack_0) (`Timeline|Timeline_0` :!via `PlayFromStart`)
    (:`Update`
      (`SceneComponent.K2_SetRelativeTransform` (`self.StaticMesh`) (`KismetMathLibrary.MakeTransform` (`KismetMathLibrary.MakeVector` (+ (`KismetMathLibrary.FClamp` (* 100 _newtrack_0) 0.0 62.0) -30.0)) (`KismetMathLibrary.MakeRotator` 0.0 _newtrack_0) (0.25 0.25 0.25)) false false)
      (if (> _newtrack_0 10.0)
        (`ActorComponent.Activate` (`self.Niagara`) false)))
    (:`Finished`
      (`self.K2_DestroyActor`))))

(fn `UserConstructionScript`
  (`parent.UserConstructionScript`))