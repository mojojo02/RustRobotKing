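; Electric child variant of the main combo actor that plays a short visual and sound effect when PlayAnim is triggered.
; It plays the Electric sound in 2D and runs a timeline that drives the static mesh's X offset and uniform scale at a fixed rotation.
; The track value is multiplied and clamped so both quickly saturate, and the actor destroys itself when the timeline finishes.
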(event `self.PlayAnim`
  (`GameplayStatics.PlaySound2D` "/Game/music/Sound/electric.electric" 1.0 1.0 0.0 null null)
  (bind (_direction _newtrack_0) (`Timeline|Timeline_0` :!via `PlayFromStart`)
    (:`Update`
      (bind _returnvalue (`KismetMathLibrary.FClamp` (* 500 _newtrack_0)))
      (`SceneComponent.K2_SetRelativeTransform` (`self.StaticMesh`) (`KismetMathLibrary.MakeTransform` (`KismetMathLibrary.MakeVector` (+ (`KismetMathLibrary.FClamp` (* 500 _newtrack_0) 0.0 100.0) 0.0) 0.0 -20.0) (`KismetMathLibrary.MakeRotator` 180.0 90.0 -15.0) (`KismetMathLibrary.MakeVector` _returnvalue _returnvalue _returnvalue)) false false))
    (:`Finished`
      (`self.K2_DestroyActor`))))

(fn `UserConstructionScript`
  (`parent.UserConstructionScript`))