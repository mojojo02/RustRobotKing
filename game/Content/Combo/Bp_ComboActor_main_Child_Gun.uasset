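; Gun variant of the combo actor that plays a one-shot gun animation with beam effect and light, then destroys itself.
; PlayAnim tints the Niagara effect, sets its beam end, and starts a timeline that slides and pitches the mesh while nudging the effect along X.
; Once the track value exceeds a threshold, the effect activates and the point light switches on; otherwise the light stays dark.
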(event `self.PlayAnim`
  (bind _niagara (`self.Niagara`))
  (bind _niagara_2 (`self.Niagara`))
  (bind _relativelocation_x (`KismetMathLibrary.BreakVector` (`SceneComponent.RelativeLocation` _niagara_2)))
  (`FXSystemComponent.SetColorParameter` _niagara "Color" (struct :`R` 0.036748 :`B` 1.0 :`A` 1.0))
  (`FXSystemComponent.SetVectorParameter` _niagara "BeanEnd" (200.0 -10.0 0.0))
  (bind (_direction _newtrack_0) (`Timeline|Timeline_0` :!via `PlayFromStart`)
    (:`Update`
      (bind _returnvalue (* 500 _newtrack_0))
      (`SceneComponent.K2_SetRelativeTransform` (`self.StaticMesh`) (`KismetMathLibrary.MakeTransform` (`KismetMathLibrary.MakeVector` (+ (`KismetMathLibrary.FClamp` _returnvalue 0.0 232.0) -200.0) 0.0 -20.0) (`KismetMathLibrary.MakeRotator` 0.0 _newtrack_0) (0.5 0.5 0.5)) false false)
      (`SceneComponent.K2_SetRelativeLocation` _niagara_2 (`KismetMathLibrary.MakeVector` (+ _relativelocation_x (`KismetMathLibrary.FClamp` _returnvalue 0.0 10.0)) -40.0) false false)
      (if (> _newtrack_0 10.0)
        (`ActorComponent.Activate` _niagara_2 false)
        (`LightComponent.SetIntensity` (`self.PointLight`) 5000.0)
        (else
          (`LightComponent.SetIntensity` (`self.PointLight`) 0.0))))
    (:`Finished`
      (`self.K2_DestroyActor`))))

(fn `UserConstructionScript`
  (`parent.UserConstructionScript`))