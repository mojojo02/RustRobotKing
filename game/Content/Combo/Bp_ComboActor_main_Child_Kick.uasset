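; Combo actor child for a kick attack, derived from the main combo actor Blueprint.
; PlayAnim plays a metal hit sound and runs a timeline that slides the static mesh along relative X and Y from a single track, keeping Z.
; The actor destroys itself when the timeline finishes, and its construction script only calls the parent's.
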(event `self.PlayAnim`
  (bind _staticmesh (`self.StaticMesh`))
  (bind (_relativelocation_x _relativelocation_y _relativelocation_z) (`KismetMathLibrary.BreakVector` (`SceneComponent.RelativeLocation` _staticmesh)))
  (`GameplayStatics.PlaySound2D` "/Game/music/Sound/metalhit.metalhit" 1.0 1.0 0.0 null null)
  (bind (_direction _newtrack_0) (`Timeline|test` :!via `PlayFromStart`)
    (:`Update`
      (`SceneComponent.K2_SetRelativeLocation` _staticmesh (`KismetMathLibrary.MakeVector` (+ _newtrack_0 50.0) (/ (+ _newtrack_0 70.0) -4.0) _relativelocation_z) false false))
    (:`Finished`
      (`self.K2_DestroyActor`))))

(fn `UserConstructionScript`
  (`parent.UserConstructionScript`))