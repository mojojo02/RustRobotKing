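; Combo-unlock tile that displays the key text of a combo from a data table row and requires the player to perform it.
; Entering while the tile is locked puts BP_Player in battle, fades the combat widget and registers the tile with the player.
; PerformCombo matches by name: success removes the cube and prompt and ends battle, failure refills action points.
; Leaving always clears battle state, also refilling points if still locked.
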(event `self.ReceiveBeginPlay`
  (`parent.ReceiveBeginPlay`)
  (bind _returnvalue (`|GetDataTableRow` "/Game/Combo/ComboDataTable.ComboDataTable" (`self.RowToComboToTest`))
    (:`then`
      (bind _output_get (set `self.ComboToPerform` _returnvalue))
      (bind _returnvalue_2 (`|CreateWidget` "/Game/Ux/ComboToUnlockInputWidget.ComboToUnlockInputWidget_C" null (`KismetTextLibrary.Conv_TextToString` (`.KeyText_35_6BA4622D4CEA67E4E35970BC349026F0` (break `/Game/Combo/ComboStruct` _output_get)))))
      (`WidgetComponent.SetWidget` (`self.Widget`) _returnvalue_2))))

(event `self.EnterPlayerCollision`
  (`parent.EnterPlayerCollision`)
  (if (`self.ISToggleCombat`)
    (bind _asbp_player (cast `/Game/BluePrintActors/Player/BP_Player_Auto1` (`GameplayStatics.GetPlayerCharacter` 0)))
    (set `/Game/BluePrintActors/Player/BP_Player_Auto1.IsInBattle?` true _asbp_player)
    (`/Game/Ux/UserCombat_widget.PlayFade` (`/Game/BluePrintActors/Player/BP_Player_Auto1.Combat_widget` _asbp_player))
    (set `/Game/BluePrintActors/Player/BP_Player_Auto1.TileComboUnlock` self _asbp_player)))

(event `self.ExitPlayerCollision`
  (`parent.ExitPlayerCollision`)
  (bind _asbp_player (cast `/Game/BluePrintActors/Player/BP_Player_Auto1` (`GameplayStatics.GetPlayerCharacter` 0)))
  (set `/Game/BluePrintActors/Player/BP_Player_Auto1.IsInBattle?` false _asbp_player)
  (if (`self.ISToggleCombat`)
    (`/Game/Ux/UserCombat_widget.PlayFade` (`/Game/BluePrintActors/Player/BP_Player_Auto1.Combat_widget` _asbp_player))
    (bind _asbp_player_2 (cast `/Game/BluePrintActors/Player/BP_Player_Auto1` (`GameplayStatics.GetPlayerCharacter` 0)))
    (set `/Game/BluePrintActors/Player/BP_Player_Auto1.CurrentActionPoints` (`/Game/BluePrintActors/Player/BP_Player_Auto1.MaxActionPoints` _asbp_player_2) _asbp_player_2)))

(event `Perform Combo`
  (params (NewParam :type "/Game/Combo/ComboStruct Structure"))
  (bind (_combotoperform_keyneeded _combotoperform_name) (break `/Game/Combo/ComboStruct` (`self.ComboToPerform`)))
  (if (`KismetTextLibrary.EqualEqual_TextText` NewParam_Name_34_2072E88E4B32408D1111EA8196A0E9FA _combotoperform_name)
    (`ActorComponent.K2_DestroyComponent` (`self.Cube`))
    (`ActorComponent.K2_DestroyComponent` (`self.Widget`))
    (set `self.ISToggleCombat` false)
    (bind _asbp_player (cast `/Game/BluePrintActors/Player/BP_Player_Auto1` (`GameplayStatics.GetPlayerCharacter` 0)))
    (set `/Game/BluePrintActors/Player/BP_Player_Auto1.IsInBattle?` false _asbp_player)
    (`/Game/Ux/UserCombat_widget.PlayFade` (`/Game/BluePrintActors/Player/BP_Player_Auto1.Combat_widget` _asbp_player))
    (else
      (bind _asbp_player_2 (cast `/Game/BluePrintActors/Player/BP_Player_Auto1` (`GameplayStatics.GetPlayerCharacter` 0)))
      (set `/Game/BluePrintActors/Player/BP_Player_Auto1.CurrentActionPoints` (`/Game/BluePrintActors/Player/BP_Player_Auto1.MaxActionPoints` _asbp_player_2) _asbp_player_2))))

(fn `UserConstructionScript`
  (`parent.UserConstructionScript`))