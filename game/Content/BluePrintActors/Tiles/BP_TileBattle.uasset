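; BP_TileBattle is a trigger tile that starts a turn-based room battle when the player enters it.
; One-time setup shares manager references, registers room tiles, instantiates enemies, puts the player in battle and starts the first turn.
; Entry also disables setup on sister battle tiles and closes their gates, so only one starts the fight.
; Doors snap between positions: closing after a delay (also on sphere overlap), reopening via FinishBattle or OpenAllGate.
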(event `self.EnterPlayerCollision`
  (`parent.EnterPlayerCollision`)
  (`self.InitialSetUp`)
  (for _array_element (`self.BpTileBattleSister`)
    (`self.DisableSetUp` _array_element)
    (`self.CloseAllGate` _array_element)))

(event `InitialSetUp`
  (bind _asbp_player (cast `/Game/BluePrintActors/Player/BP_Player_Auto1` (`GameplayStatics.GetPlayerCharacter` 0) :!pure true))
  ;[1 1 1] Player Enter colision Générate array of all tile and put Ref of ennemies + cast anim en bool of player
  (`/Engine/EditorBlueprintResources/StandardMacros.DoOnce` (`self.CloseDoOnce`)
    (:`Completed`
      ;[0 0.2388 1] Begin Play Initalize all ref
      (for _array_element (`self.Tiles`)
        (`KismetArrayLibrary.Array_Add` (`self.TilesPosition`) (`SceneComponent.K2_GetComponentLocation` (`/Game/BluePrintActors/Tiles/BP_Tile.CollisonSphere` _array_element)))
        (for _array_element_2 (`self.Enemies`)
          (set `/Game/BluePrintActors/Enemies/BP_Enemy.BP_BattleManagerRef` (`self.BattleManagerRef`) _array_element_2)
          (set `/Game/BluePrintActors/Enemies/BP_Enemy.BP_TilesManagerRef` (`self.BP_TilesManagerRef`) _array_element_2))
        (set `/Game/BluePrintActors/Managers/BP_BattleManager.BP_TilesManagerRef` (`self.BP_TilesManagerRef`) (`self.BattleManagerRef`)))
      (set `/Game/BluePrintActors/Player/BP_Player_Auto1.BattleManageur` (`self.BattleManagerRef`) _asbp_player)
      (set `/Game/BluePrintActors/Player/BP_Player_Auto1.TileManager` (`self.BP_TilesManagerRef`) _asbp_player)
      (`/Game/BluePrintActors/Managers/BP_TilesManager.GetAllRoomTiles` (`self.BP_TilesManagerRef`) (`self.TilesPosition`) (`self.Tiles`))
      (`/Game/BluePrintActors/Managers/BP_BattleManager.InstantiateEnemies` (`self.BattleManagerRef`) (`self.Enemies`))
      (bind _asbp_player_2 (cast `/Game/BluePrintActors/Player/BP_Player_Auto1` (`GameplayStatics.GetPlayerCharacter` 0)))
      (`/Game/BluePrintActors/Player/BP_Player_Auto1.EnterBattle` _asbp_player_2)
      (`/Game/BluePrintActors/Managers/BP_BattleManager.SetNextTurn` (`self.BattleManagerRef`)))))

(event `DisableSetUp`
  ;[1 1 1] Player Enter colision Générate array of all tile and put Ref of ennemies + cast anim en bool of player
  (set `self.CloseDoOnce` true))

(event `self.ExitPlayerCollision`
  (`parent.ExitPlayerCollision`))

(event `FinishBattle`
  (`SceneComponent.K2_SetRelativeLocation` (`self.Door`) (0.0 100.0 400.0) false false))

(event `CloseAllGate`
  (`/Engine/EditorBlueprintResources/StandardMacros.DoOnce` false :!label _label
    (:`Completed`
      (`KismetSystemLibrary.Delay` 1.0)
      (`SceneComponent.K2_SetRelativeLocation` (`self.Door`) (0.0 100.0 100.0) false false)
      (`GameplayStatics.PlaySoundAtLocation` "/Game/music/Sound/doorclosing.doorclosing" (`SceneComponent.K2_GetComponentLocation` (`self.Door`)) (struct) 1.0 1.0 0.0 null null null))))

(event `self.CollisonSphere.OnComponentBeginOverlap`
  (params (OverlappedComponent :type "PrimitiveComponent Object Reference") (OtherActor :type "Actor Object Reference") (OtherComp :type "PrimitiveComponent Object Reference") (OtherBodyIndex :type Integer) (bFromSweep :type Boolean) (SweepResult :type "HitResult Structure (by ref)"))
  (goto _label))

(event `OpenAllGate`
  (`SceneComponent.K2_SetRelativeLocation` (`self.Door`) (0.0 100.0 400.0) false false)
  (`GameplayStatics.PlaySoundAtLocation` "/Game/music/Sound/dooropening.dooropening" (`SceneComponent.K2_GetComponentLocation` (`self.Door`)) (struct) 1.0 1.0 0.0 null null null))

(fn `UserConstructionScript`
  (`parent.UserConstructionScript`))