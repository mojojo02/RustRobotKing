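; BP_Tile is a board tile actor that tracks player or enemy occupancy and relays attack damage to the enemy standing on it.
; Enter and exit events update occupancy and availability flags, with the player's also toggling the collision box.
; EnableDmg briefly shows the highlight and damages any valid stored enemy, gated by a DoOnce until explicitly reset.
; It also holds G, H and F scores, suggesting A* pathfinding, summing F only at BeginPlay.
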(event `EnableDmg`
  (params (dmg :type Integer))
  (bind _ennemionref (`self.EnnemiOnRef`))
  ;[1 1 1] Enable DMG
  (`/Engine/EditorBlueprintResources/StandardMacros.DoOnce` false :!label _label
    (:`Completed`
      (`SceneComponent.SetVisibility` (`self.TileHiglight`) true false)
      (`|ExecutionSequence`
        (:`then_0`
          (if (`self.HaveEnnemi`)
            (`/Engine/EditorBlueprintResources/StandardMacros.IsValid` _ennemionref
              (:`Is Valid`
                (`/Game/BluePrintActors/Enemies/BP_Enemy.TakeDmg` _ennemionref dmg)))))
        (:`then_1`
          (`KismetSystemLibrary.Delay` 2.0)
          (`SceneComponent.SetVisibility` (`self.TileHiglight`) false false))))))

(event `ResteEnableDMG`
  ;[1 1 1] Enable DMG
  (goto _label :!via `Reset`))

(event `self.ReceiveBeginPlay`
  ;[1 1 1] Begin Play
  (set `self.F` (+ (`self.G`) (`self.H`))))

(event `EnnemiExit`
  ;[1 1 1] Ennemi go in / out
  (set `self.HaveEnnemi` false)
  (set `self.IsAvaible` true))

(event `Ennemi Enter`
  (params (EnnemiOnRef :type "/Game/BluePrintActors/Enemies/BP_Enemy Object Reference"))
  ;[1 1 1] Ennemi go in / out
  (set `self.EnnemiOnRef` EnnemiOnRef)
  (set `self.HaveEnnemi` true)
  (set `self.IsAvaible` false))

(event `EnterPlayerCollision`
  ;[1 1 1] Player go in / out
  (set `self.HavePlayer` true)
  (`PrimitiveComponent.SetCollisionEnabled` (`self.CollisionBox`) "NoCollision")
  (set `self.IsAvaible` false))

(event `ExitPlayerCollision`
  ;[1 1 1] Player go in / out
  (set `self.HavePlayer` false)
  (`PrimitiveComponent.SetCollisionEnabled` (`self.CollisionBox`) "QueryAndPhysics")
  (set `self.IsAvaible` true))

(fn `UserConstructionScript`)