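; Player controller that turns directional key presses into grid-style movement calls outside battle and combo input during battle.
; In battle, keys are buffered within a cooldown window and a four-key cap, shown on the combat widget, with action-point cost gated by a flag.
; A retriggerable delay fires the combo once input pauses, mapping keys to direction enums for BP_Player's ApplyCombo and clearing the buffer.
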(event `PerformForwardInput`
  (params (`Axis Value` :type Integer) (`Key Pressed` :type "Key Structure" :default "None"))
  ;[1 1 1] ForwardInputs
  (bind _asbp_player (cast `/Game/BluePrintActors/Player/BP_Player_Auto1` (`GameplayStatics.GetPlayerCharacter` 0)))
  (if (not (`/Game/BluePrintActors/Player/BP_Player_Auto1.IsPerformedACombo` _asbp_player))
    (if (`/Game/BluePrintActors/Player/BP_Player_Auto1.IsInBattle?` _asbp_player)
      (`self.AddKeyToCombo` `Key Pressed`)
      (if (`self.IsNotMaxKey`)
        (`/Game/BluePrintActors/Player/BP_Player_Auto1.RemoveActionPoints` _asbp_player 1))
      (else
        (`/Game/BluePrintActors/Player/BP_Player_Auto1.ForwardMove` _asbp_player `Axis Value`)))))

(event `InputAction|ForwardMovementUp`
  (params (Key :type "Key Structure"))
  ;[1 1 1] ForwardInputs
  (:`Pressed`
    (`self.PerformForwardInput` 1 Key)))

(event `InputAction|ForwardMovementDown`
  (params (Key :type "Key Structure"))
  ;[1 1 1] ForwardInputs
  (:`Pressed`
    (`self.PerformForwardInput` -1 Key)))

(event `PerformSideInput`
  (params (AxisValue :type Integer) (KeyPressed :type "Key Structure" :default "None"))
  ;[1 1 1] SideInputs
  (bind _asbp_player (cast `/Game/BluePrintActors/Player/BP_Player_Auto1` (`GameplayStatics.GetPlayerCharacter` 0)))
  (if (not (`/Game/BluePrintActors/Player/BP_Player_Auto1.IsPerformedACombo` _asbp_player))
    (if (`/Game/BluePrintActors/Player/BP_Player_Auto1.IsInBattle?` _asbp_player)
      (`self.AddKeyToCombo` KeyPressed)
      (if (`self.IsNotMaxKey`)
        (`/Game/BluePrintActors/Player/BP_Player_Auto1.RemoveActionPoints` _asbp_player 1))
      (else
        (`/Game/BluePrintActors/Player/BP_Player_Auto1.SideMove` _asbp_player AxisValue)))))

(event `InputAction|LeftRotation`
  (params (Key :type "Key Structure"))
  ;[1 1 1] SideInputs
  (:`Pressed`
    (`self.PerformSideInput` -1 Key)))

(event `InputAction|RightRotation`
  (params (Key :type "Key Structure"))
  ;[1 1 1] SideInputs
  (:`Pressed`
    (`self.PerformSideInput` 1 Key)))

(event `AddKeyToCombo`
  (params (KeyPressed :type "Key Structure" :default "None"))
  ;[1 1 1] Combo Logic
  (if (== (`KismetArrayLibrary.Array_Length` (`self.Inputs`)) 0)
    (`KismetArrayLibrary.Array_Add` (`self.Inputs`) KeyPressed)
    (set `self.LastInputTime` (`KismetSystemLibrary.GetGameTimeInSeconds`))
    (`/Game/Ux/UserCombat_widget.UpdateKeyText` (`/Game/BluePrintActors/Player/BP_Player_Auto1.Combat_widget` (cast `/Game/BluePrintActors/Player/BP_Player_Auto1` (`GameplayStatics.GetPlayerCharacter` 0) :!pure true)) KeyPressed :!label _label)
    (`self.CheckExecuteCombo`)
    (else
      (`self.CheckMAxEnterKey`
        (:`true`
          (if (<= (- (`KismetSystemLibrary.GetGameTimeInSeconds`) (`self.LastInputTime`)) (`self.InputCooldown`))
            (set `self.LastInputTime` (`KismetSystemLibrary.GetGameTimeInSeconds`))
            (`KismetArrayLibrary.Array_Add` (`self.Inputs`) KeyPressed)
            (goto _label)))))))

(event `PerformCombo`
  (bind _returnvalue (`GameplayStatics.GetPlayerController` 0))
  ;[1 1 1] Perform Combo Logic
  (`self.DisableInput` _returnvalue null)
  (for _array_element (`self.Inputs`)
    (if (`self.CheckKeyName` _array_element "w" "up")
      (bind _output_get (set `self.KeyEnum` "NewEnumerator0"))
      (`KismetArrayLibrary.Array_Add` (`self.KeyPerformed`) _output_get)
      (elif (`self.CheckKeyName` _array_element "s" "down")
        (bind _output_get_2 (set `self.KeyEnum` "NewEnumerator1"))
        (`KismetArrayLibrary.Array_Add` (`self.KeyPerformed`) _output_get_2)
        (elif (`self.CheckKeyName` _array_element "a" "left")
          (bind _output_get_3 (set `self.KeyEnum` "NewEnumerator3"))
          (`KismetArrayLibrary.Array_Add` (`self.KeyPerformed`) _output_get_3)
          (elif (`self.CheckKeyName` _array_element "d" "right")
            (bind _output_get_4 (set `self.KeyEnum` "NewEnumerator2"))
            (`KismetArrayLibrary.Array_Add` (`self.KeyPerformed`) _output_get_4))))))
  (`/Game/BluePrintActors/Player/BP_Player_Auto1.ApplyCombo` (cast `/Game/BluePrintActors/Player/BP_Player_Auto1` (`GameplayStatics.GetPlayerCharacter` 0) :!pure true) (`self.KeyPerformed`))
  (`KismetArrayLibrary.Array_Clear` (`self.KeyPerformed`))
  (`self.EnableInput` _returnvalue null))

(event `CheckExecuteCombo`
  ;[1 1 1] Check if must perform combo
  ;;[1 1 1] Patching this issue !
  (`KismetSystemLibrary.RetriggerableDelay` (`self.InputCooldown`))
  (set `self.IsNotMaxKey` false)
  (`self.PerformCombo`)
  (`KismetArrayLibrary.Array_Clear` (`self.Inputs`)))

(fn `UserConstructionScript`)