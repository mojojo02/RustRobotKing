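; Player pawn for a tile-based, turn-based combat game, handling grid movement, health, action points, potion inventory, music and UI.
; Entered key sequences are matched against a combo DataTable; otherwise they replay as timed steps, with line traces finding the next tile.
; A matched combo spawns an attack actor and briefly enables damage on a width-by-depth area of tiles ahead via TileManager.
; Running out of action points passes the turn to the battle manager.
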(event `Ambiance`
  (`/Engine/EditorBlueprintResources/StandardMacros.FlipFlop`
    (:`A`
      (bind _returnvalue (`GameplayStatics.SpawnSound2D` "/Game/music/music/ambience2.ambience2" 1.0 1.0 0.0 null))
      (bind _output_get (set `self.Sound` _returnvalue))
      (`ActorComponent.Activate` _output_get false))
    (:`B`
      (bind _returnvalue_2 (`GameplayStatics.SpawnSound2D` "/Game/music/music/ambientsounds.ambientsounds" 1.0 1.0 0.0 null))
      (bind _output_get_2 (set `self.Sound` _returnvalue_2))
      (`ActorComponent.Activate` _returnvalue_2 false)
      (`ActorComponent.Activate` _output_get_2 false))))

(event `Add Combo`
  (params (RowName :type Name))
  ;[1 1 1] Add combo
  (bind _returnvalue (`|GetDataTableRow` "/Game/Combo/ComboDataTable.ComboDataTable" RowName)
    (:`then`
      (`KismetArrayLibrary.Array_AddUnique` (`self.ComboOwned`) _returnvalue)
      (`/Game/Ux/UserCombat_widget.UpdateCombo` (`self.Combat_widget`)))))

(event `Key|P`
  (params (Key :type "Key Structure"))
  (:`Pressed`
    (`self.OptionWidget` :!label _label)))

(event `OptionWidget`
  (`/Engine/EditorBlueprintResources/StandardMacros.FlipFlop`
    (:`A`
      (bind _returnvalue (`|CreateWidget` "/Game/Ux/OptionWidget.OptionWidget_C"))
      (`UserWidget.AddToViewport` _returnvalue 0)
      (set `self.Option Wdget` _returnvalue))
    (:`B`
      (`Widget.RemoveFromParent` (`self.Option Wdget`)))))

(event `Key|Escape`
  (params (Key :type "Key Structure"))
  (:`Pressed`
    (goto _label)))

(event `self.ReceiveBeginPlay`
  ;[0 0.1815 1] Event begin play
  (`WidgetBlueprintLibrary.SetInputMode_GameAndUIEx` (`GameplayStatics.GetPlayerController` 0) null)
  (set `self.IsInBattle?` false)
  (set `self.CurrentHealthPoints` (`self.MaxHealthPoints`))
  (set `self.CurrentActionPoints` (`self.MaxActionPoints`))
  (bind _returnvalue (`|CreateWidget` "/Game/Ux/UserCombat_widget.UserCombat_widget_C"))
  (`UserWidget.AddToViewport` _returnvalue 0)
  (set `self.Combat_widget` _returnvalue)
  (set `PlayerController.bShowMouseCursor` true (`GameplayStatics.GetPlayerController` 0))
  (bind _asbp_player_controller (cast `/Game/BluePrintActors/Player/BP_PlayerController_Auto3` (`GameplayStatics.GetPlayerController` 0)))
  (`/Game/BluePrintActors/Player/BP_PlayerController_Auto3.PerformForwardInput` _asbp_player_controller 1 "W")
  (`self.Add Combo` "Kick")
  (`UserWidget.PlayAnimationReverse` _returnvalue (`/Game/Ux/UserCombat_widget.fade` _returnvalue) 1.0 false)
  (`self.Ambiance`))

(event `ForwardMove`
  (params (InputAxisValue :type Integer))
  (bind _bp_tileref (`self.BP_TileRef`))
  (bind _capsulecomponent (`self.CapsuleComponent`))
  (bind _returnvalue (`SceneComponent.K2_GetComponentLocation` _capsulecomponent))
  ;[1 1 1] Forward Movement
  (bind (_outhit _returnvalue_2) (`KismetSystemLibrary.LineTraceSingle` _returnvalue (+ (* (* (`SceneComponent.GetForwardVector` _capsulecomponent) InputAxisValue) (1000.0 1000.0 0.0)) _returnvalue) "TraceTypeQuery1"))
  (if _returnvalue_2
    (bind _asbp_tile (cast `/Game/BluePrintActors/Tiles/BP_Tile` (`.HitActor` (`GameplayStatics.BreakHitResult` _outhit))))
    (if (`/Game/BluePrintActors/Tiles/BP_Tile.IsAvaible` _asbp_tile)
      (`/Engine/EditorBlueprintResources/StandardMacros.IsValid` _bp_tileref
        (:`Is Valid`
          (`/Game/BluePrintActors/Tiles/BP_Tile.ExitPlayerCollision` _bp_tileref))
        (:`Is Not Valid`
          _))
      (bind _output_get (set `self.BP_TileRef` _asbp_tile))
      (`/Game/BluePrintActors/Tiles/BP_Tile.EnterPlayerCollision` _output_get)
      (`SceneComponent.K2_SetWorldLocation` (`self.CapsuleComponent`) (`SceneComponent.K2_GetComponentLocation` (`/Game/BluePrintActors/Tiles/BP_Tile.CollisonSphere` _asbp_tile)) true false))))

(event `SideMove`
  (params (InputAxisValue :type Integer))
  ;[1 1 1] Side Rotation Movement Logic
  (`SceneComponent.K2_SetWorldRotation` (`self.CapsuleComponent`) (`KismetMathLibrary.ComposeRotators` (`SceneComponent.K2_GetComponentRotation` (`self.CapsuleComponent`)) (`KismetMathLibrary.MakeRotator` 0.0 0.0 (`KismetMathLibrary.Conv_IntToDouble` (* InputAxisValue 90)))) false false))

(event `EnterBattle`
  ;[1 1 1] Battle anim logic
  (set `self.IsInBattle?` true)
  (`/Game/Ux/UserCombat_widget.PlayFade` (`self.Combat_widget`))
  (`ActorComponent.K2_DestroyComponent` (`self.Sound`))
  (bind _returnvalue (`GameplayStatics.SpawnSound2D` "/Game/music/music/Fight_music2.Fight_music2" 1.0 1.0 0.0 null))
  (bind _output_get (set `self.Sound` _returnvalue))
  (`ActorComponent.Activate` _output_get false))

(event `FinishBattle`
  ;[1 1 1] Battle anim logic
  (`GameplayStatics.PlaySound2D` "/Game/music/Sound/win.win" 1.0 1.0 0.0 null null)
  (`WidgetBlueprintLibrary.SetInputMode_GameAndUIEx` (`GameplayStatics.GetPlayerController` 0) null)
  (set `self.IsInBattle?` false)
  (`/Game/Ux/UserCombat_widget.PlayFade` (`self.Combat_widget`))
  (`ActorComponent.K2_DestroyComponent` (`self.Sound`))
  (`self.Ambiance`))

(event `AddBuff`
  (params (dmgBuffer :type "Float (double-precision)"))
  ;[1 1 1] Add DmgBuff
  (set `self.DmgBuffer` dmgBuffer))

(event `UpdateItemInventory`
  (params (itemRef :type "/Game/item/ItemStruct Structure"))
  (bind _iteminventorystruct (`self.ItemInventoryStruct`))
  (bind _returnvalue (`KismetArrayLibrary.Array_Find` _iteminventorystruct itemRef))
  ;[1 1 1] Item Update Information
  (set `self.IndexUpdateItem` _returnvalue)
  (bind _result (`/Engine/EditorBlueprintResources/StandardMacros.DecrementInt` (`.Ammount_9_09847DF642D1AE7E11DECCABAE9EEA8E` (break `/Game/item/ItemStruct` (`|GetArrayItem` _iteminventorystruct _returnvalue))))
    (:`  `
      (if (== _result 0)
        (`KismetArrayLibrary.Array_Remove` (`self.ItemInventoryStruct`) (`self.IndexUpdateItem`))
        (`/Game/Ux/UserCombat_widget.UpdateListe` (`self.Combat_widget`))))))

(event `AddItemInventory`
  (params (ItemStruct :type "/Game/item/ItemStruct Structure"))
  (bind (_ammount _potiontype) (break `/Game/item/ItemStruct` ItemStruct))
  ;[1 1 1] Add logic
  (set `self.IsSameObject` false)
  (for (_array_element _array_index) (`self.ItemInventoryStruct`)
    (if (`|EnumEquality` (`.PotionType_6_07B5939B491FD286F1BF9383A50E13BE` (break `/Game/item/ItemStruct` _array_element)) _potiontype)
      (set `self.IsSameObject` true)
      (bind _ammount_2 (break `/Game/item/ItemStruct` (`|GetArrayItem` (`self.ItemInventoryStruct`) _array_index)))
      (`/Engine/EditorBlueprintResources/StandardMacros.ManipulateIntInternal` _ammount_2 (+ _ammount_2 _ammount)
        (:`  `
          (break)))))
  (if (not (`self.IsSameObject`))
    (`KismetArrayLibrary.Array_Add` (`self.ItemInventoryStruct`) ItemStruct))
  (`/Game/Ux/UserCombat_widget.UpdateListe` (`self.Combat_widget`)))

(event `TakeDamage`
  (params (Damage :type Integer))
  (bind _maxhealthpoints (`self.MaxHealthPoints`))
  (bind _currenthealthpoints (`self.CurrentHealthPoints`))
  (bind _returnvalue (- (`self.CurrentHealthPoints`) Damage))
  ;[1 1 1] Take Damage Logic
  (`GameplayStatics.PlaySound2D` "/Game/music/Sound/robotdie.robotdie" 1.0 2.0 0.0 null null)
  (if (not (<= _returnvalue 0))
    (if (not (> _returnvalue (`self.MaxHealthPoints`)))
      (set `self.CurrentHealthPoints` _returnvalue)
      (else
        (set `self.CurrentHealthPoints` _maxhealthpoints)))
    (`/Game/Ux/UserCombat_widget.Update Health` (`self.Combat_widget`) (/ (`KismetMathLibrary.Conv_IntToDouble` _currenthealthpoints) (`KismetMathLibrary.Conv_IntToDouble` _maxhealthpoints)) _currenthealthpoints)
    (else
      (`ActorComponent.K2_DestroyComponent` (`self.Sound`))
      (bind _returnvalue_2 (`|CreateWidget` "/Game/Ux/LoosWidget.LoosWidget_C"))
      (`UserWidget.AddToViewport` _returnvalue_2 0)
      (`GameplayStatics.SetGamePaused` true))))

(event `RemoveActionPoints`
  (params (nbrToRemove :type Integer))
  (bind _maxactionpoints (`self.MaxActionPoints`))
  (bind _currentactionpoints (`self.CurrentActionPoints`))
  (bind _returnvalue (- (`self.CurrentActionPoints`) nbrToRemove))
  ;[1 1 1] Remove Action Points Logic
  (if (not (> _returnvalue _maxactionpoints))
    (bind _output_get (set `self.CurrentActionPoints` _returnvalue))
    ;;[1 1 1] Temp Befor Turn/Turn
    (if (== _output_get 0)
      (`WidgetBlueprintLibrary.SetInputMode_UIOnlyEx` (`GameplayStatics.GetPlayerController` 0) null))
    (else
      (set `self.CurrentActionPoints` _maxactionpoints)))
  (`/Game/Ux/UserCombat_widget.UpdateAp` (`self.Combat_widget`) (/ (`KismetMathLibrary.Conv_IntToDouble` _currentactionpoints) (`KismetMathLibrary.Conv_IntToDouble` _maxactionpoints)) _currentactionpoints))

(event `ApplyCombo`
  (params (KeyPerformed :type "Array of /Game/Combo/KeyEnum Enum"))
  (bind _capsulecomponent (`self.CapsuleComponent`))
  (bind _tilemanager (`self.TileManager`))
  (bind (_keyneeded _name _keytext _tile_width _tile_depth _dammage _actortospawn) (break `/Game/Combo/ComboStruct` (`self.ComboToExecute`)))
  (bind _returnvalue (`SceneComponent.K2_GetComponentLocation` _capsulecomponent))
  (bind _returnvalue_2 (- _tile_depth 1))
  ;[1 1 1] ComboApplyLogic
  (set `self.Key Performed` KeyPerformed)
  (set `self.IsPerformedACombo` true)
  ;;[0 0.1469 1] Check Is a combo
  (bind _outrownames (`DataTableFunctionLibrary.GetDataTableRowNames` "/Game/Combo/ComboDataTable.ComboDataTable"))
  (for _array_element _outrownames
    (bind _returnvalue_3 (`|GetDataTableRow` "/Game/Combo/ComboDataTable.ComboDataTable" _array_element)
      (:`then`
        (if (`KismetArrayLibrary.Array_Identical` (`self.Key Performed`) (`.KeyNeeded_14_E80A67164A284389183BADBA76145A8B` (break `/Game/Combo/ComboStruct` _returnvalue_3)))
          (set `self.ComboToExecute` _returnvalue_3)
          (set `self.ComboExist` true)
          (break)
          (else
            (set `self.ComboExist` false))))))
  (if (`self.ComboExist`)
    ;;[0.955 0 1] A combo
    (`KismetArrayLibrary.Array_AddUnique` (`self.ComboOwned`) (`self.ComboToExecute`))
    (`/Game/Ux/UserCombat_widget.UpdateCombo` (`self.Combat_widget`))
    (bind _outhit (`KismetSystemLibrary.LineTraceSingle` :`Start` _returnvalue :`End` (+ (* (`SceneComponent.GetForwardVector` _capsulecomponent) (1000.0 1000.0 0.0)) _returnvalue) :`TraceChannel` "TraceTypeQuery1" :`TraceColor` (struct :`G` 1.0 :`B` 0.129762 :`A` 1.0) :`TraceHitColor` (struct :`R` 0.974049 :`B` 1.0 :`A` 1.0)))
    (bind _asbp_tile (cast `/Game/BluePrintActors/Tiles/BP_Tile` (`.HitActor` (`GameplayStatics.BreakHitResult` _outhit)))
      (:`then`
        (set `self.DammageToApply` _dammage)
        (for _index (range _tile_width)
          (bind _returnvalue_4 (`SceneComponent.K2_GetComponentLocation` (`/Game/BluePrintActors/Tiles/BP_Tile.CollisonSphere` _asbp_tile)))
          (bind _returnvalue_5 (* (* (200.0 200.0 0.0) _index) (`KismetMathLibrary.Cross_VectorVector` (`SceneComponent.GetForwardVector` (`self.CapsuleComponent`)) (1.0 1.0 1.0))))
          (bind _tile (`/Game/BluePrintActors/Managers/BP_TilesManager.GetTileAtPosition` _tilemanager (+ _returnvalue_4 _returnvalue_5)))
          (`/Engine/EditorBlueprintResources/StandardMacros.IsValid` _tile
            (:`Is Valid`
              (`KismetArrayLibrary.Array_Add` (`self.AllTileTakeDmg`) _tile)
              (`|ExecutionSequence`
                (:`then_0`
                  (`self.FoorLoopDepthTile` _returnvalue_2 _tile (`self.DammageToApply`)))
                (:`then_1`
                  (`/Game/BluePrintActors/Tiles/BP_Tile.EnableDmg` _tile (`self.DammageToApply`))
                  (bind _tile_2 (`/Game/BluePrintActors/Managers/BP_TilesManager.GetTileAtPosition` _tilemanager (- _returnvalue_4 _returnvalue_5) :!label _label_2))
                  (`/Engine/EditorBlueprintResources/StandardMacros.IsValid` _tile_2
                    (:`Is Valid`
                      (`KismetArrayLibrary.Array_Add` (`self.AllTileTakeDmg`) _tile_2)
                      (`/Game/BluePrintActors/Tiles/BP_Tile.EnableDmg` _tile_2 (`self.DammageToApply`))
                      (`self.FoorLoopDepthTile` _returnvalue_2 _tile_2 (`self.DammageToApply`)))))))
            (:`Is Not Valid`
              (goto _label_2)))))
      (:`CastFailed`
        _))
    (bind _returnvalue_6 (`|SpawnActorFromClass` _actortospawn (`KismetMathLibrary.MakeTransform` (`SceneComponent.K2_GetComponentLocation` (`self.Sphere`)) (`SceneComponent.K2_GetComponentRotation` (`self.CapsuleComponent`))) "Undefined" "OverrideRootScale" null null))
    (`/Game/Combo/Bp_ComboActor_main.PlayAnim` _returnvalue_6)
    (`KismetSystemLibrary.Delay` 0.2)
    (for _array_element_2 (`self.AllTileTakeDmg`)
      (`/Game/BluePrintActors/Tiles/BP_Tile.ResteEnableDMG` _array_element_2))
    (`KismetArrayLibrary.Array_Clear` (`self.AllTileTakeDmg`))
    (`/Game/Ux/UserCombat_widget.ClearKeyText` (`self.Combat_widget`) :!label _label_3)
    (set `/Game/BluePrintActors/Player/BP_PlayerController_Auto3.IsNotMaxKey` true (cast `/Game/BluePrintActors/Player/BP_PlayerController_Auto3` (`GameplayStatics.GetPlayerController` 0) :!pure true))
    (set `self.IsPerformedACombo` false)
    (if (== (`self.CurrentActionPoints`) 0)
      (`self.TurnOver`))
    (else
      ;;[0 0.1098 1] Not a combo
      (bind _arrayelem (`/Game/CustomLoop.ForEachLoopDelay` (`self.Key Performed`) 0.5)
        (:`update`
          (switch `/Game/Combo/KeyEnum` _arrayelem
            (:`NewEnumerator0`
              (`self.ForwardMove` 1))
            (:`NewEnumerator1`
              (`self.ForwardMove` -1))
            (:`NewEnumerator2`
              (`self.SideMove` 1))
            (:`NewEnumerator3`
              (`self.SideMove` -1))))
        (:`Completed`
          (goto _label_3))))))

(event `StartTurn`
  (bind _currentactionpoints (`self.CurrentActionPoints`))
  ;[1 1 1] Start turn Logic
  (set `self.CurrentActionPoints` (`self.MaxActionPoints`))
  (`WidgetBlueprintLibrary.SetInputMode_GameAndUIEx` (`GameplayStatics.GetPlayerController` 0) null "DoNotLock" false)
  (`/Game/Ux/UserCombat_widget.UpdateAp` (`self.Combat_widget`) (/ (`KismetMathLibrary.Conv_IntToDouble` _currentactionpoints) (`KismetMathLibrary.Conv_IntToDouble` (`self.MaxActionPoints`))) _currentactionpoints)
  (`/Game/Ux/UserCombat_widget.EnableButton` (`self.Combat_widget`)))

(event `TurnOver`
  ;[1 1 1] Start turn Logic
  (`WidgetBlueprintLibrary.SetInputMode_UIOnlyEx` (`GameplayStatics.GetPlayerController` 0) null)
  (`/Game/BluePrintActors/Managers/BP_BattleManager.SetNextTurn` (`self.BattleManageur`))
  (`/Game/Ux/UserCombat_widget.DisableButton` (`self.Combat_widget`)))

(fn `UserConstructionScript`)