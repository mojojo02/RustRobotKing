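; Turn-based grid enemy that snaps to a tile, then spends action points each turn approaching and attacking the player.
; StartTurn runs an A*-style tile search (G and H both measure from the start), trimming the path by AP and, for ranged units, row/column alignment.
; Delayed steps feed tile positions to the behavior tree's blackboard; leftover AP drives montage attacks.
; The battle manager receives turn ends and deaths.
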(event `self.ReceivePossessed`
  (params (NewController :type "Controller Object Reference"))
  (`AIController.RunBehaviorTree` (`AIBlueprintHelperLibrary.GetAIController` self) "/Game/BluePrintActors/Enemies/BT_Enemy_2.BT_Enemy_2")
  (`BlackboardComponent.SetValueAsObject` (`AIBlueprintHelperLibrary.GetBlackboard` null) "EnemyActor" (`self.BP_PlayerRef`)))

(event `self.ReceiveBeginPlay`
  (bind _capsulecomponent (`self.CapsuleComponent`))
  (bind _returnvalue (`SceneComponent.K2_GetComponentLocation` _capsulecomponent))
  ;[0 0.1327 1] More profitable tu put inside TileBattlerButUsless
  (bind _asbp_player (cast `/Game/BluePrintActors/Player/BP_Player_Auto1` (`GameplayStatics.GetPlayerCharacter` 0)))
  (set `self.BP_PlayerRef` _asbp_player)
  (bind (_outhit _returnvalue_2) (`KismetSystemLibrary.LineTraceSingle` _returnvalue (+ (* (`SceneComponent.GetForwardVector` _capsulecomponent) (1000.0 1000.0 0.0)) _returnvalue) "TraceTypeQuery1"))
  (if _returnvalue_2
    (bind _asbp_tile (cast `/Game/BluePrintActors/Tiles/BP_Tile` (`.HitActor` (`GameplayStatics.BreakHitResult` _outhit))))
    (if (`/Game/BluePrintActors/Tiles/BP_Tile.IsAvaible` _asbp_tile)
      (`/Game/BluePrintActors/Tiles/BP_Tile.Ennemi Enter` _asbp_tile self)
      (bind _output_get (set `self.TileRef` _asbp_tile))
      (`SceneComponent.K2_SetWorldLocation` (`self.CapsuleComponent`) (`SceneComponent.K2_GetComponentLocation` (`/Game/BluePrintActors/Tiles/BP_Tile.CollisonSphere` _output_get)) false true))))

(event `StartTurn`
  (bind _currentap (`self.CurrentAp`))
  (bind _tileref (`self.TileRef`))
  (bind _returnvalue (`KismetArrayLibrary.Array_Length` (`self.Path`)))
  (bind (_returnvalue_x _returnvalue_y) (`KismetMathLibrary.BreakVector` (`SceneComponent.K2_GetComponentLocation` (`/Game/BluePrintActors/Tiles/BP_Tile.CollisonSphere` (`/Game/BluePrintActors/Player/BP_Player_Auto1.BP_TileRef` (`self.BP_PlayerRef`))))))
  ;[1 0.07275 0] StartTurn
  (`/Game/BluePrintActors/Tiles/BP_Tile.EnterPlayerCollision` _tileref)
  (`/Game/BluePrintActors/Tiles/BP_Tile.EnnemiExit` _tileref)
  (set `self.CurrentAp` (`self.MaxAp`))
  (bind _path (`self.FindPath` (`SceneComponent.K2_GetComponentLocation` (`/Game/BluePrintActors/Tiles/BP_Tile.CollisonSphere` (`self.TileRef`))) (`SceneComponent.K2_GetComponentLocation` (`/Game/BluePrintActors/Tiles/BP_Tile.CollisonSphere` (`/Game/BluePrintActors/Player/BP_Player_Auto1.BP_TileRef` (cast `/Game/BluePrintActors/Player/BP_Player_Auto1` (`GameplayStatics.GetPlayerCharacter` 0) :!pure true))))))
  (bind _output_get (set `self.Path` _path))
  ;;[1 1 1] case du joueur
  (`KismetArrayLibrary.Array_Remove` _output_get (`KismetArrayLibrary.Array_LastIndex` _output_get))
  (if (not (== (`self.Range`) 0))
    ;;[1 1 1] RangeLOgic
    (for _index (range (`KismetMathLibrary.Clamp` (- _returnvalue (`self.Range`)) 0 100) (+ _returnvalue 1))
      (bind (_output_x _output_y) (`KismetMathLibrary.BreakVector` (`|GetArrayItem` (`self.Path`) _index)))
      (if (or (== _output_x _returnvalue_x) (== _output_y _returnvalue_y))
        (`KismetArrayLibrary.Array_Resize` (`self.Path`) (+ _index 1))
        (break))))
  (bind _returnvalue_2 (`KismetArrayLibrary.Array_Length` _output_get))
  (if (> _currentap _returnvalue_2)
    (set `self.CurrentAp` (- _currentap _returnvalue_2))
    (else
      (`KismetArrayLibrary.Array_Resize` (`self.Path`) _currentap)
      (set `self.CurrentAp` 0)))
  (bind _arrayelem (`/Game/CustomLoop.ForEachLoopDelay` (`self.Path`) 1.0)
    (:`update`
      ;;[1 1 1] MoveTile Logic
      (bind (_outhit _returnvalue_3) (`KismetSystemLibrary.LineTraceSingle` (`SceneComponent.K2_GetComponentLocation` (`self.CapsuleComponent`)) _arrayelem "TraceTypeQuery1"))
      (if _returnvalue_3
        (`/Game/BluePrintActors/Tiles/BP_Tile.ExitPlayerCollision` (`self.TileRef`))
        (bind _asbp_tile (cast `/Game/BluePrintActors/Tiles/BP_Tile` (`.HitActor` (`GameplayStatics.BreakHitResult` _outhit))))
        (bind _output_get_2 (set `self.TileRef` _asbp_tile))
        (`/Game/BluePrintActors/Tiles/BP_Tile.EnterPlayerCollision` _output_get_2)
        (`BlackboardComponent.SetValueAsVector` (`AIBlueprintHelperLibrary.GetBlackboard` null) "PostionToMove" (`SceneComponent.K2_GetComponentLocation` (`/Game/BluePrintActors/Tiles/BP_Tile.CollisonSphere` _output_get_2)))
        (else
          (`KismetSystemLibrary.PrintString` "Ennemy is stuck because anavaible tile"))))
    (:`Completed`
      ;;[1 1 1] SwitchBetweenAction
      (if (> (`self.CurrentAp`) 0)
        (`self.Attack`)
        (else
          (`self.FinishTurn`))))))

(event `Attack`
  ;[1 1 1] Faudrait-il ajouter un systeme d'esquive ???
  (`/Game/BluePrintActors/Macros/CustomLoop.ForLoopDelay` 0 (`self.CurrentAp`) 2.0
    (:`Loop`
      (`self.PlayAnimMontage` (`self.AttackMontage`))
      (`/Game/BluePrintActors/Player/BP_Player_Auto1.TakeDamage` (`self.BP_PlayerRef`) (`self.Degat`)))
    (:`Over`
      (`self.FinishTurn`))))

(event `FinishTurn`
  (bind _tileref (`self.TileRef`))
  ;[1 1 1] Finish Turn
  (`/Game/BluePrintActors/Tiles/BP_Tile.ExitPlayerCollision` _tileref)
  (`/Game/BluePrintActors/Tiles/BP_Tile.Ennemi Enter` _tileref self)
  (`/Game/BluePrintActors/Managers/BP_BattleManager.SetNextTurn` (`self.BP_BattleManagerRef`)))

(event `TakeDmg`
  (params (dmg :type Integer))
  (bind _returnvalue (- (`self.Hp`) dmg))
  ;[1 1 1] TakeDmg
  (if (<= _returnvalue 0)
    (`/Game/BluePrintActors/Managers/BP_BattleManager.RemoveEnemies` (`self.BP_BattleManagerRef`) self)
    (`/Game/BluePrintActors/Tiles/BP_Tile.EnnemiExit` (`self.TileRef`))
    (`PrimitiveComponent.SetCollisionEnabled` (`self.CapsuleComponent`) "NoCollision")
    (`ActorComponent.Activate` (`self.DieEmitter`) true)
    (bind _returnvalue_2 (`self.PlayAnimMontage` (`self.DieMontage`)))
    (`KismetSystemLibrary.Delay` (- _returnvalue_2 0.5))
    (`self.K2_DestroyActor`)
    (else
      (set `self.Hp` _returnvalue))))

(fn `FindPath`
  (params (StartPos :type "Vector Structure") (EndPos :type "Vector Structure"))
  (returns (path :type "Array of Vector Structure"))
  (locals (OpenList :type "Array of Vector Structure") (ClosedList :type "Array of Vector Structure") (F_Array :type "Array of Integer") (currentPos :type "Vector Structure") (OpenListTiles :type "Array of /Game/BluePrintActors/Tiles/BP_Tile Object Reference") (ClosedListTiles :type "Array of /Game/BluePrintActors/Tiles/BP_Tile Object Reference") (Direction :type "Array of Vector Structure") (neighbor :type "Vector Structure") (StartPosFindPath :type "Vector Structure") (EndPosFindPath :type "Vector Structure"))
  (bind _openlisttiles (`local.OpenListTiles`))
  (set `local.StartPosFindPath` StartPos)
  (set `local.EndPosFindPath` EndPos)
  ;[1 1 1] On récupère la tile sur laquelle on est
  (bind _tile (`/Game/BluePrintActors/Managers/BP_TilesManager.GetTileAtPosition` (`self.BP_TilesManagerRef`) (`local.StartPosFindPath`)))
  ;[1 1 1] on l'ajoute à notre liste
  (`KismetArrayLibrary.Array_Add` _openlisttiles _tile)
  (while (> (`KismetArrayLibrary.Array_Length` _openlisttiles) 0)
    ;[1 1 1] Je suis pas sûre de l'intéret car là à chaque itération du while on récupère notre position actuel
    (bind _outarray (`self.SortArray` (`local.OpenListTiles`)))
    ;;[1 1 1] Et on regard la tuile
    (bind _output_get (set `local.currentPos` (`SceneComponent.K2_GetComponentLocation` (`/Game/BluePrintActors/Tiles/BP_Tile.CollisonSphere` (`|GetArrayItem` _outarray)))))
    (bind _tile_2 (`/Game/BluePrintActors/Managers/BP_TilesManager.GetTileAtPosition` (`self.BP_TilesManagerRef`) _output_get))
    ;[1 1 1] Et on retire notre postion ?
    (`KismetArrayLibrary.Array_RemoveItem` (`local.OpenListTiles`) _tile_2)
    ;[1 1 1] Pour l'ajouter dans closed liste tile
    (`KismetArrayLibrary.Array_Add` (`local.ClosedListTiles`) _tile_2)
    ;[1 1 1] On regard si on a atteint la cible
    (if (== (`local.currentPos`) (`local.EndPosFindPath`))
      ;[1 1 1] Si oui alors on retourne le chemin
      (bind _finishereversedlist (`self.Restructure Path` (`local.StartPosFindPath`) (`local.EndPosFindPath`)))
      (return _finishereversedlist)
      (else
        ;[1 1 1] On éffectue ce check pour chaque direction (chaque tile voisine)
        ;;[1 1 1] Si non alors on observe toutes les tile à côté
        (for _array_element (`local.Direction`)
          (set `local.neighbor` (+ (`local.currentPos`) _array_element))
          ;;[1 1 1] On vérifie si elles sont valide
          (bind _isposavailable_ (`self.IsPositionAvailable` (`local.neighbor`)))
          ;;[1 1 1] On récupe l'info de la tile
          (bind _tile_3 (`/Game/BluePrintActors/Managers/BP_TilesManager.GetTileAtPosition` (`self.BP_TilesManagerRef`) (`local.neighbor`)))
          (if (not (or (== _isposavailable_ false) (`KismetArrayLibrary.Array_Contains` (`local.ClosedListTiles`) _tile_3)))
            ;[1 0 0] On l'a déjà fais ça ...
            (bind _tile_4 (`/Game/BluePrintActors/Managers/BP_TilesManager.GetTileAtPosition` (`self.BP_TilesManagerRef`) (`local.neighbor`)))
            ;[1 1 1] On regard la distance les séparant
            (bind _int (`self.GetMathanttenDistance` (`local.StartPosFindPath`) (`local.neighbor`)))
            (set `/Game/BluePrintActors/Tiles/BP_Tile.G` _int _tile_4)
            ;[1 0 0] On l'a déjà fais ???
            (bind _tile_5 (`/Game/BluePrintActors/Managers/BP_TilesManager.GetTileAtPosition` (`self.BP_TilesManagerRef`) (`local.neighbor`)))
            ;[1 1 1] Je comprend pas on a deja fais ça, aucun paramètre n'a changé pk le mettre sur H (que signifie g et H ? )
            (bind _int_2 (`self.GetMathanttenDistance` (`local.StartPosFindPath`) (`local.neighbor`)))
            (set `/Game/BluePrintActors/Tiles/BP_Tile.H` _int_2 _tile_5)
            ;[1 0 0] Ok définitevement un mistère
            (bind _tile_6 (`/Game/BluePrintActors/Managers/BP_TilesManager.GetTileAtPosition` (`self.BP_TilesManagerRef`) (`local.neighbor`)))
            ;[1 1 1] On récup l'info de notre position
            (bind _tile_7 (`/Game/BluePrintActors/Managers/BP_TilesManager.GetTileAtPosition` (`self.BP_TilesManagerRef`) (`local.currentPos`)))
            ;[1 1 1] Ok donc on dis au voisin que notre case actuel était la derniÈre
            (set `/Game/BluePrintActors/Tiles/BP_Tile.BP_PreviousTile` _tile_7 _tile_6)
            ;[1 1 1] Pk ne pas avoir promote neigboor pose à une variable ?
            (bind _tile_8 (`/Game/BluePrintActors/Managers/BP_TilesManager.GetTileAtPosition` (`self.BP_TilesManagerRef`) (`local.neighbor`)))
            (if (not (`KismetArrayLibrary.Array_Contains` (`local.OpenListTiles`) _tile_8))
              (`KismetArrayLibrary.Array_Add` (`local.OpenListTiles`) _tile_8)
              (else
                (`KismetSystemLibrary.PrintString` "Dans Find Path BpEnnemy : la tuile exsitait déjà dans l'open List !" true true (struct :`R` 0.940283 :`G` 1.0 :`A` 1.0)))))))))
  (`KismetSystemLibrary.PrintString` "In Find path BpEnnemy : the length of open tile was 0" true true (struct :`R` 0.098097 :`G` 1.0 :`A` 1.0))
  (`KismetSystemLibrary.PrintString` "Hello")
  (return (`self.Path`)))

(fn `FindPathDijkstra`)

(fn `GetAvailableTiles`
  (params (StartPos :type "Vector Structure") (Range :type Integer))
  (returns (AvailableTiles :type "Map of Vector Structure to Integer"))
  (locals (tmpArrayL :type "Array of Vector Structure") (AvailableTilesL :type "Map of Vector Structure to Object Object Reference") (CurrentPosL :type "Vector Structure") (DirectionsL :type "Array of Vector Structure") (NeighborL :type "Vector Structure"))
  (bind _tmparrayl (`local.tmpArrayL`))
  (bind _tmparrayl_2 (`local.tmpArrayL`))
  (`BlueprintMapLibrary.Map_Add` (`local.AvailableTilesL`) StartPos)
  (`KismetArrayLibrary.Array_Add` _tmparrayl_2 StartPos)
  (while (> (`KismetArrayLibrary.Array_Length` _tmparrayl_2) 0)
    (bind _output_get (set `local.CurrentPosL` (`|GetArrayItem` _tmparrayl)))
    (`KismetArrayLibrary.Array_RemoveItem` _tmparrayl _output_get)
    (for _array_element (`local.DirectionsL`)
      (bind _output_get_2 (set `local.NeighborL` (+ (`local.CurrentPosL`) _array_element)))
      (bind _isposavailable_ (`self.IsPositionAvailable` _output_get_2))
      (if (and _isposavailable_ (not (`BlueprintMapLibrary.Map_Contains` (`local.AvailableTilesL`) _output_get_2)))
        (bind _returnvalue (+ (`BlueprintMapLibrary.Map_Find` (`local.AvailableTilesL`) _output_get) 1))
        (if (<= _returnvalue Range)
          (`BlueprintMapLibrary.Map_Add` (`local.AvailableTilesL`) _output_get_2 _returnvalue)
          (`KismetArrayLibrary.Array_Add` (`local.tmpArrayL`) _output_get_2))))
    (`KismetSystemLibrary.PrintString` "Fin "))
  (return (`local.AvailableTilesL`)))

(fn `GetMathanttenDistance`
  (params (StartPos :type "Vector Structure") (neighborPos :type "Vector Structure"))
  (returns (int :type Integer))
  (return (+ (`KismetMathLibrary.Abs_Int` (- (`KismetMathLibrary.FFloor` (.x StartPos)) (`KismetMathLibrary.FFloor` (.x neighborPos)))) (`KismetMathLibrary.Abs_Int` (- (`KismetMathLibrary.FFloor` (.y StartPos)) (`KismetMathLibrary.FFloor` (.y neighborPos)))))))

(fn `IsPositionAvailable`
  (params (position :type "Vector Structure"))
  (returns (`IsPosAvailable?` :type Boolean))
  (bind _bp_tilesmanagerref (`self.BP_TilesManagerRef`))
  (bind _tile (`/Game/BluePrintActors/Managers/BP_TilesManager.GetTileAtPosition` _bp_tilesmanagerref position))
  (`/Engine/EditorBlueprintResources/StandardMacros.IsValid` _tile
    (:`Is Valid`
      (return (and (`KismetArrayLibrary.Array_Contains` (`/Game/BluePrintActors/Managers/BP_TilesManager.TilesPosition` _bp_tilesmanagerref) position) (or (`/Game/BluePrintActors/Tiles/BP_Tile.IsAvaible` _tile) (`/Game/BluePrintActors/Tiles/BP_Tile.HavePlayer` _tile)))))
    (:`Is Not Valid`
      (return false))))

(fn `Restructure Path`
  (params (StartPos :type "Vector Structure") (EndPos :type "Vector Structure"))
  (returns (FinisheReversedList :type "Array of Vector Structure"))
  (locals (finishedList :type "Array of Vector Structure") (CurrentPos :type "Vector Structure"))
  (set `local.CurrentPos` EndPos)
  (while (!= (`local.CurrentPos`) StartPos)
    (`KismetArrayLibrary.Array_Add` (`local.finishedList`) (`local.CurrentPos`))
    (bind _tile (`/Game/BluePrintActors/Managers/BP_TilesManager.GetTileAtPosition` (`self.BP_TilesManagerRef`) (`local.CurrentPos`)))
    (set `local.CurrentPos` (`SceneComponent.K2_GetComponentLocation` (`/Game/BluePrintActors/Tiles/BP_Tile.CollisonSphere` (`/Game/BluePrintActors/Tiles/BP_Tile.BP_PreviousTile` _tile)))))
  (`KismetArrayLibrary.Array_Reverse` (`local.finishedList`))
  (return (`local.finishedList`)))

(fn `SortArray`
  (params (Tiles :type "Array of /Game/BluePrintActors/Tiles/BP_Tile Object Reference"))
  (returns (OutArray :type "Array of /Game/BluePrintActors/Tiles/BP_Tile Object Reference"))
  (locals (tmpArray :type "Array of /Game/BluePrintActors/Tiles/BP_Tile Object Reference") (`tmp Elements` :type Integer) (`In Array` :type "Array of /Game/BluePrintActors/Tiles/BP_Tile Object Reference") (`Tmp Actor` :type "/Game/BluePrintActors/Tiles/BP_Tile Object Reference") (`Tmp F Distance Array` :type "Array of Integer") (`Tmp Found Index` :type Integer) (`Tmp Out Array` :type "Array of /Game/BluePrintActors/Tiles/BP_Tile Object Reference"))
  (set `local.tmpArray` Tiles)
  (set `local.tmp Elements` (`KismetArrayLibrary.Array_LastIndex` Tiles))
  (bind _arrayelementref (`/Game/BluePrintActors/Macros/CustomRefLoop.ForEachRefLoop` Tiles)
    (:`Update`
      (bind _output_get (set `local.Tmp Actor` _arrayelementref))
      (bind _output_get_2 (set `/Game/BluePrintActors/Tiles/BP_Tile.F` (+ (`/Game/BluePrintActors/Tiles/BP_Tile.G` _output_get) (`/Game/BluePrintActors/Tiles/BP_Tile.H` _output_get)) _output_get))
      (`KismetArrayLibrary.Array_Add` (`local.Tmp F Distance Array`) _output_get_2))
    (:`Complete`
      (for _ (range (+ (`local.tmp Elements`) 1))
        (bind _output_get_3 (set `local.Tmp Found Index` (`KismetMathLibrary.MinOfIntArray` (`local.Tmp F Distance Array`))))
        (`KismetArrayLibrary.Array_Add` (`local.Tmp Out Array`) (`|GetArrayItem` (`local.tmpArray`) _output_get_3))
        (`KismetArrayLibrary.Array_Remove` (`local.Tmp F Distance Array`) (`local.Tmp Found Index`))
        (`KismetArrayLibrary.Array_Remove` (`local.tmpArray`) (`local.Tmp Found Index`)))
      (return (`local.Tmp Out Array`)))))

(fn `SortArrayByInt`
  (params (`Int Array` :type "Array of Integer") (Tiles :type "Array of /Game/BluePrintActors/Tiles/BP_Tile Object Reference"))
  (returns (Sorted :type "Array of Integer") (SortedOldIndex :type "Array of Integer"))
  (locals (`Array Int Val` :type "Array of Integer") (`Array Old Index` :type "Array of Integer") (`Sorted Array` :type "Array of Integer") (`F_Tiles Array` :type "Array of Integer"))
  (bind _array_int_val (`local.Array Int Val`))
  (bind (_indexofminvalue _minvalue) (`KismetMathLibrary.MinOfIntArray` _array_int_val))
  (for (_array_element _array_index) Tiles
    (`KismetArrayLibrary.Array_Set` (`local.F_Tiles Array`) _array_index (`/Game/BluePrintActors/Tiles/BP_Tile.F` _array_element))
    (for (_array_element_2 _array_index_2) `Int Array`
      (`KismetArrayLibrary.Array_Set` (`local.Array Int Val`) _array_index_2 _array_element_2 true))
    (for _index (range (+ (`KismetArrayLibrary.Array_LastIndex` `Int Array`) 1))
      (`KismetArrayLibrary.Array_Set` (`local.Array Old Index`) _index _indexofminvalue true)
      (`KismetArrayLibrary.Array_Set` (`local.Sorted Array`) _index _minvalue true)
      (`KismetArrayLibrary.Array_Set` _array_int_val _indexofminvalue (+ (`.MaxValue` (`KismetMathLibrary.MaxOfIntArray` `Int Array`)) 1)))
    (return (`local.Sorted Array`) (`local.Array Old Index`))))

(fn `UserConstructionScript`)