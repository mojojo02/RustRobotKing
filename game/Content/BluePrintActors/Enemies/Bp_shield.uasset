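; Shield-bearing enemy Blueprint that sets its own stats and montages on top of a parent class and blocks head-on damage.
; TakeDmg compares its capsule's forward vector with the player's reversed one; a near match negates the hit and plays a Timeline that shifts the shield.
; Other hits reduce Hp, and a lethal one removes it from the battle manager, disables collision, plays death effects, then destroys it.
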(event `self.ReceiveBeginPlay`
  (`parent.ReceiveBeginPlay`)
  (set `self.Hp` 200)
  (set `self.Range` 0)
  (set `self.MaxAp` 3)
  (set `self.Degat` 30)
  (set `self.AttackMontage` "/Game/EnnemiMesh/Shield/anim/ShitldAttack_Montage.ShitldAttack_Montage")
  (set `self.DieMontage` "/Game/EnnemiMesh/Shield/anim/ShieldDie_Montage.ShieldDie_Montage"))

(event `self.TakeDmg`
  (params (dmg :type Integer))
  (bind _returnvalue (- (`self.Hp`) dmg))
  (if (not (== (`SceneComponent.GetForwardVector` (`self.CapsuleComponent`)) (* (`SceneComponent.GetForwardVector` (`Character.CapsuleComponent` (`self.BP_PlayerRef`))) -1) :`ErrorTolerance` 0.1))
    (if (<= _returnvalue 0)
      (`KismetArrayLibrary.Array_RemoveItem` (`/Game/BluePrintActors/Managers/BP_BattleManager.Enemies` (`self.BP_BattleManagerRef`)) self)
      (`PrimitiveComponent.SetCollisionEnabled` (`self.CapsuleComponent`) "NoCollision")
      (`ActorComponent.Activate` (`self.DieEmitter`) true)
      (bind _returnvalue_2 (`self.PlayAnimMontage` (`self.DieMontage`)))
      (`KismetSystemLibrary.Delay` (- _returnvalue_2 0.5))
      (`self.K2_DestroyActor`)
      (else
        (set `self.Hp` _returnvalue)))
    (else
      (bind (_direction _newtrack_0) (`Timeline|Timeline_0` :!via `PlayFromStart`)
        (:`Update`
          (`SceneComponent.K2_SetRelativeLocation` (`self.Shield`) (`KismetMathLibrary.MakeVector` _newtrack_0) false false))))))

(fn `UserConstructionScript`
  (`parent.UserConstructionScript`))