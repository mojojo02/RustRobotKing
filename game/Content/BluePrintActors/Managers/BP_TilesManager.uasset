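; BP_TilesManager is a manager Blueprint that holds a room's tiles and looks them up by world position.
; The GetAllRoomTiles event receives and stores the tile positions and tile references.
; GetTileAtPosition linearly searches the stored tiles for one whose collision sphere location nearly exactly matches the given position, printing a debug error when none matches.
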(event `GetAllRoomTiles`
  (params (TilesPosition :type "Array of Vector Structure") (Tiles :type "Array of /Game/BluePrintActors/Tiles/BP_Tile Object Reference"))
  (set `self.TilesPosition` TilesPosition)
  (set `self.Tiles` Tiles))

(fn `GetTileAtPosition`
  (params (position :type "Vector Structure"))
  (returns (tile :type "/Game/BluePrintActors/Tiles/BP_Tile Object Reference"))
  (bind _arrayelementref (`/Game/BluePrintActors/Macros/CustomRefLoop.ForEachRefLoop` (`self.Tiles`))
    (:`Update`
      (if (== (`SceneComponent.K2_GetComponentLocation` (`/Game/BluePrintActors/Tiles/BP_Tile.CollisonSphere` _arrayelementref)) position)
        (return _arrayelementref)))
    (:`Complete`
      (`KismetSystemLibrary.PrintString` "ErrorInGetTilePostionBpEnnemi : i'm not on a valide tile" true true (struct :`R` 0.99373 :`B` 1.0 :`A` 1.0)))))

(fn `UserConstructionScript`)