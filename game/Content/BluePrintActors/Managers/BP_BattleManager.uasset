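; BP_BattleManager runs turn-based battles, cycling turns between the player and a list of enemies.
; InstantiateEnemies sets the list, and SetNextTurn increments a counter, using modulo to start the player's turn or the matching enemy's.
; Enemy removal and each turn change check for an empty list, which opens all BP_TileBattle gates, calls the player's FinishBattle and resets turn and tile-manager data.
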(event `RemoveEnemies`
  (params (Enemy :type "/Game/BluePrintActors/Enemies/BP_Enemy Object Reference"))
  (bind _bp_tilesmanagerref (`self.BP_TilesManagerRef`))
  (`KismetArrayLibrary.Array_RemoveItem` (`self.Enemies`) Enemy)
  (if (== (`KismetArrayLibrary.Array_Length` (`self.Enemies`)) 0) :!label _label
    (bind _outactors (`GameplayStatics.GetAllActorsOfClass` "/Game/BluePrintActors/Tiles/BP_TileBattle.BP_TileBattle_C"))
    (for _array_element _outactors
      (`/Game/BluePrintActors/Tiles/BP_TileBattle.OpenAllGate` _array_element))
    (`/Game/BluePrintActors/Player/BP_Player_Auto1.FinishBattle` (cast `/Game/BluePrintActors/Player/BP_Player_Auto1` (`GameplayStatics.GetPlayerCharacter` 0) :!pure true))
    (`KismetArrayLibrary.Array_Clear` (`self.Enemies`))
    (set `self.CurrentTurn` -1)
    (`KismetArrayLibrary.Array_Clear` (`/Game/BluePrintActors/Managers/BP_TilesManager.Tiles` _bp_tilesmanagerref))
    (`KismetArrayLibrary.Array_Clear` (`/Game/BluePrintActors/Managers/BP_TilesManager.TilesPosition` _bp_tilesmanagerref))))

(event `InstantiateEnemies`
  (params (Enemies :type "Array of /Game/BluePrintActors/Enemies/BP_Enemy Object Reference"))
  (set `self.Enemies` Enemies))

(event `SetNextTurn`
  (bind _returnvalue (mod (`self.CurrentTurn`) (+ (`KismetArrayLibrary.Array_Length` (`self.Enemies`)) 1)))
  (`|ExecutionSequence`
    (:`then_0`
      (goto _label))
    (:`then_1`
      (`/Engine/EditorBlueprintResources/StandardMacros.IncrementInt` (`self.CurrentTurn`)
        (:`  `
          (if (== _returnvalue 0)
            (bind _asbp_player (cast `/Game/BluePrintActors/Player/BP_Player_Auto1` (`GameplayStatics.GetPlayerCharacter` 0)))
            (`/Game/BluePrintActors/Player/BP_Player_Auto1.StartTurn` _asbp_player)
            (else
              (`/Game/BluePrintActors/Enemies/BP_Enemy.StartTurn` (`|GetArrayItem` (`self.Enemies`) (- _returnvalue 1))))))))))

(fn `UserConstructionScript`)